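; Dollar bill actor Blueprint that implements a VR grip interface, with no gameplay logic of its own.
; Free and slot grips both use interactive collision with physics, with late updates always on and original movement replication kept.
; Grip slot searches always report none in range, gripping is not denied, and double grip and simulate-on-drop are off.
; Event graph and construction script are empty.
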(fn `CanHaveDoubleGrip`
  (returns (ReturnValue :type Boolean))
  (return false))

(fn `ClosestPrimarySlotInRange`
  (params (WorldLocation :type "Vector Structure"))
  (returns (bHadSlotInRange :type Boolean) (SlotWorldTransform :type "Transform Structure"))
  (return false))

(fn `ClosestSecondarySlotInRange`
  (params (WorldLocation :type "Vector Structure"))
  (returns (bHadSlotInRange :type Boolean) (SlotWorldTransform :type "Transform Structure"))
  (return false))

(fn `DenyGripping`
  (returns (ReturnValue :type Boolean))
  (return false))

(fn `FreeGripType`
  (returns (ReturnValue :type "EGripCollisionType Enum"))
  (return "InteractiveCollisionWithPhysics"))

(fn `GetInteractionSettings`
  (returns (ReturnValue :type "BPInteractionSettings Structure"))
  (return))

(fn `GripBreakDistance`
  (returns (ReturnValue :type "Float (double-precision)"))
  (return 0.0))

(fn `GripDamping`
  (returns (ReturnValue :type "Float (double-precision)"))
  (return 0.0))

(fn `GripLateUpdateSetting`
  (returns (ReturnValue :type "EGripLateUpdateSettings Enum"))
  (return "LateUpdatesAlwaysOn"))

(fn `GripMovementReplicationType`
  (returns (ReturnValue :type "EGripMovementReplicationSettings Enum"))
  (return "KeepOriginalMovement"))

(fn `GripStiffness`
  (returns (ReturnValue :type "Float (double-precision)"))
  (return 0.0))

(fn `IsHeld`
  (returns (HoldingController :type "GripMotionControllerComponent Object Reference") (bIsHeld :type Boolean))
  (return null false))

(fn `IsInteractible`
  (returns (ReturnValue :type Boolean))
  (return false))

(fn `ObjectType`
  (returns (ObjectType :type Byte))
  (return 0))

(fn `SimulateOnDrop`
  (returns (ReturnValue :type Boolean))
  (return false))

(fn `SlotGripType`
  (returns (ReturnValue :type "EGripCollisionType Enum"))
  (return "InteractiveCollisionWithPhysics"))

(fn `TeleportBehavior`
  (returns (ReturnValue :type "EGripInterfaceTeleportBehavior Enum"))
  (return "TeleportAllComponents"))

(fn `UserConstructionScript`)